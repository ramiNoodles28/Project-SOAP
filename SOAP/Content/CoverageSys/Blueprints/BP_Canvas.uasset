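; BP_Canvas is a paintable surface actor that records brush marks in a render target shown through its mesh material.
; Each tick it traces below the player, paints any canvas hit at its collision UV, and reports the impact point to BP_ThirdPersonGameMode.
; Splash traces vertically around a world position to paint at a given radius.
; Paint's Dirty flag only selects which material receives the brush texture; drawing always uses BrushMat.
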(event `self.ReceiveBeginPlay`
  (`|ExecutionSequence`
    (:`then_0`
      (bind _returnvalue (`KismetRenderingLibrary.CreateRenderTarget2D` 4096 4096))
      (bind _output_get (set `self.RenderTarget` _returnvalue))
      (`KismetRenderingLibrary.ClearRenderTarget2D` _output_get (struct :`R` 0.208333 :`G` 0.208333 :`B` 0.208333 :`A` 1.0)))
    (:`then_1`
      (bind _returnvalue_2 (`KismetMaterialLibrary.CreateDynamicMaterialInstance` "/Game/CoverageSys/Materials_Textures/M_Canvas.M_Canvas"))
      (`MaterialInstanceDynamic.SetTextureParameterValue` _returnvalue_2 "RenderTarget" (`self.RenderTarget`))
      (`PrimitiveComponent.SetMaterial` (`self.CanvasMesh`) 0 _returnvalue_2))
    (:`then_2`
      (bind _returnvalue_3 (`KismetMaterialLibrary.CreateDynamicMaterialInstance` "/Game/CoverageSys/Materials_Textures/M_Brush.M_Brush"))
      (set `self.BrushMat` _returnvalue_3))
    (:`then_3`
      (bind _returnvalue_4 (`KismetMaterialLibrary.CreateDynamicMaterialInstance` "/Game/CoverageSys/Materials_Textures/M_Brush_Dirty.M_Brush_Dirty"))
      (set `self.BrushMat_D` _returnvalue_4))))

(event `self.ReceiveTick`
  (params (DeltaSeconds :type "Float (single-precision)"))
  (bind _returnvalue (`self.K2_GetActorLocation` (`GameplayStatics.GetPlayerCharacter` 0)))
  (bind _outhit (`KismetSystemLibrary.LineTraceSingle` :`Start` (+ _returnvalue (`KismetMathLibrary.MakeVector` 0.0 0.0 -90.1)) :`End` (+ _returnvalue (`KismetMathLibrary.MakeVector` 0.0 0.0 -93.0)) :`TraceChannel` "TraceTypeQuery1" :`bTraceComplex` true :`bIgnoreSelf` false))
  (bind (_bblockinghit _binitialoverlap _time _distance _location _impactpoint _normal _impactnormal _physmat _hitactor) (`GameplayStatics.BreakHitResult` _outhit))
  (bind _asbp_canvas (cast `/Game/CoverageSys/Blueprints/BP_Canvas` _hitactor))
  (`|ExecutionSequence`
    (:`then_0`
      (`self.Paint` _asbp_canvas (`self.T Brush`) (`self.Brush Size`) (`GameplayStatics.FindCollisionUV` _outhit) false))
    (:`then_1`
      (bind _asbp_third_person_game_mode (cast `/Game/ThirdPerson/Blueprints/BP_ThirdPersonGameMode` (`GameplayStatics.GetGameMode`)))
      (`/Game/ThirdPerson/Blueprints/BP_ThirdPersonGameMode.HandlePaintHit` _asbp_third_person_game_mode _impactpoint))))

(fn `Paint`
  (params (T_Brush :type "Texture Object Reference") (BrushSize :type "Float (double-precision)") (DrawLocation :type "Vector2D Structure") (bDirty :type Boolean))
  (bind _brushsize (`local.BrushSize`))
  (`|ExecutionSequence`
    (:`then_0`
      (`MaterialInstanceDynamic.SetTextureParameterValue` (select `bool` bDirty :`false` (`self.BrushMat`) :`true` (`self.BrushMat_D`)) "Brush" T_Brush))
    (:`then_1`
      (bind (_canvas _size _context) (`KismetRenderingLibrary.BeginDrawCanvasToRenderTarget` (`self.RenderTarget`)))
      (`Canvas.K2_DrawMaterial` _canvas (`self.BrushMat`) (- (* _size (`local.DrawLocation`)) (/ _brushsize 2.0)) (`KismetMathLibrary.MakeVector2D` _brushsize _brushsize) (0.0 0.0) (1.0 1.0) 0.0 (0.5 0.5))
      (`KismetRenderingLibrary.EndDrawCanvasToRenderTarget` _context))))

(fn `Splash`
  (params (WorldPos :type "Vector Structure") (Radius :type "Float (double-precision)"))
  (bind (_outhit _returnvalue) (`KismetSystemLibrary.LineTraceSingle` (+ WorldPos (0.0 0.0 200.0)) (- WorldPos (0.0 0.0 800.0)) "TraceTypeQuery1" true (`|MakeArray` (`GameplayStatics.GetPlayerCharacter` 0) :!type "Actor Object Reference") "Persistent" false))
  (if _returnvalue
    (bind (_uv _returnvalue_2) (`GameplayStatics.FindCollisionUV` _outhit))
    (if _returnvalue_2
      (`self.Paint` (`self.T Brush`) Radius _uv))))

(fn `UserConstructionScript`)