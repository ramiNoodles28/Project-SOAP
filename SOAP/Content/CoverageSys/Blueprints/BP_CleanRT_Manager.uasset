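; Coverage manager actor that paints a brush into a render target at the surface UV beneath the player.
; A looping timer line-traces down through the player, converts the hit to collision UV and draws the brush dynamic material there.
; The brush material takes previous-target and mask textures, but BeginPlay leaves these and the material parent unset.
; Variable-driven setup, HUD creation and readback nodes are present but never run.
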(event `self.ReceiveBeginPlay`
  (`KismetRenderingLibrary.DrawMaterialToRenderTarget` null)
  (bind _returnvalue (`KismetMaterialLibrary.CreateDynamicMaterialInstance` null))
  (bind _output_get (set `self.BrushMID` _returnvalue))
  (`MaterialInstanceDynamic.SetTextureParameterValue` _output_get "PrevRT" null)
  (`MaterialInstanceDynamic.SetTextureParameterValue` _output_get "MaskTex" null)
  (`KismetSystemLibrary.K2_SetTimerDelegate` (delegate `PaintTick`) 0.05 true)
  (`self.PaintTick`))

(event `PaintTick`
  (bind _returnvalue (`self.K2_GetActorLocation` (`GameplayStatics.GetPlayerCharacter` 0)))
  (bind (_outhit _returnvalue_2) (`KismetSystemLibrary.LineTraceSingle` :`Start` (+ _returnvalue (`KismetMathLibrary.MakeVector` 0.0 0.0 100.0)) :`End` (+ _returnvalue (`KismetMathLibrary.MakeVector` 0.0 0.0 -500.0)) :`TraceChannel` "TraceTypeQuery1" :`bTraceComplex` true :`DrawDebugType` "Persistent"))
  (if _returnvalue_2
    (bind (_uv _returnvalue_3) (`GameplayStatics.FindCollisionUV` _outhit))
    (if _returnvalue_3
      (bind (_x _y) (`KismetMathLibrary.BreakVector2D` _uv))
      (`MaterialInstanceDynamic.SetVectorParameterValue` (`self.BrushMID`) "BrushUVCenter" (make `LinearColor` _x _y))
      (`KismetRenderingLibrary.DrawMaterialToRenderTarget` null (`self.BrushMID`))
      (else
        (`KismetSystemLibrary.PrintString` "FindCollisionUV Failed")))))

(fn `UserConstructionScript`)