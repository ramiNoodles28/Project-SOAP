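; Coverage manager that tracks how much of the level's coverage volumes has been visited and reports the overall percentage.
; While the game runs, TickManagerUpdate brushes each volume at this actor's own location, then sums allowed and visited counts into a ratio for the HUD.
; The brush loop wires back into itself, and the WBP_CleanHUD creation chain is disconnected, so HUDRef is never assigned here.
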(event `self.ReceiveBeginPlay`
  ; UI Update
)

(event `TickManagerUpdate`
  (bind _array (`|MakeArray` (`self.CoverageVolumes`)))
  ; TickManager
  (if (`self.bGameRunning`)
    (for _array_element _array :!label _label
      (`/Game/CoverageSys/Blueprints/Old/BP_CoverageVolume. BrushVisitAtWorld` _array_element (`self.K2_GetActorLocation`))
      (goto _label))
    (set `self.TotalAllowed` 0)
    (set `self.TotalVisited` 0)
    (for _array_element_2 _array
      (bind (_allowed _visited) (`/Game/CoverageSys/Blueprints/Old/BP_CoverageVolume.GetCounts` _array_element_2))
      (set `self.TotalAllowed` (+ _allowed (`self.TotalAllowed`)))
      (set `self.TotalVisited` (+ _visited (`self.TotalVisited`))))
    (if (> (`self.TotalAllowed`) 0)
      (bind _output_get (set `self.TotalCoveragePercent` (/ (`KismetMathLibrary.Conv_IntToDouble` (`self.TotalVisited`)) (`KismetMathLibrary.Conv_IntToDouble` (`self.TotalAllowed`)))))
      (`/Game/CoverageSys/Widgets/WBP_CleanHUD.SetCoveragePercent` (`self.HUDRef`) _output_get (`self.TotalVisited`) (`self.TotalAllowed`))
      (else
        (set `self.TotalCoveragePercent` 0.0)))))

(fn `UserConstructionScript`)