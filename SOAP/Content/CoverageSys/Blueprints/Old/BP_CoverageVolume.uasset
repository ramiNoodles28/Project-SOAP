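; Coverage volume that tracks how much cleanable surface inside its bounds has been visited by a circular brush.
; BuildGridAndAllowed divides the bounds into cells and line-traces each vertically, flagging hits that pass height, surface normal and optional "Cleanable" tag checks.
; BrushVisitAtWorld maps a world position to the grid and marks allowed, unvisited cells within the brush radius.
; Flat boolean masks hold cell state, with running totals exposed through GetCounts.
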(event `BuildGridAndAllowed`
  (bind _cellsize (`self.CellSize`))
  (bind (_returnvalue_x _returnvalue_y) (`KismetMathLibrary.BreakVector` (`BoxComponent.GetScaledBoxExtent` (`self.Bounds`))))
  ; Build Grid
  (bind _output_get (set `self.NumX` (`KismetMathLibrary.Max` (`KismetMathLibrary.FFloor` (/ (* _returnvalue_x 2.0) _cellsize)) 1)))
  (bind _output_get_2 (set `self.NumY` (`KismetMathLibrary.Max` (`KismetMathLibrary.FFloor` (/ (* _returnvalue_y 2.0) _cellsize)) 1)))
  (`KismetArrayLibrary.Array_Clear` (`self.AllowedMask`))
  (`KismetArrayLibrary.Array_Clear` (`self.VisitedMask`))
  (set `self.AllowedCount` 0)
  (set `self.VisitedCount` 0)
  (for _index (range _output_get_2)
    (for _index_2 (range _output_get)
      (bind _worldlocation (`self.GridIndexToWorld` _index _index_2))
      (bind (_outhit _returnvalue) (`KismetSystemLibrary.LineTraceSingle` :`Start` (+ _worldlocation (`KismetMathLibrary.MakeVector` 0.0 0.0 200.0)) :`End` (+ _worldlocation (`KismetMathLibrary.MakeVector` 0.0 0.0 -400.0)) :`TraceChannel` "TraceTypeQuery1" :`bTraceComplex` true :`DrawDebugType` "Persistent"))
      (if _returnvalue
        (bind _returnvalue_2 (`self.IsHitCleanable` _outhit))
        (if _returnvalue_2
          (`KismetArrayLibrary.Array_Set` (`self.AllowedMask`) (+ _index_2 (* _index (`self.NumX`))) true)
          (set `self.AllowedCount` (+ (`self.AllowedCount`) 1)))))))

(fn ` BrushVisitAtWorld`
  (params (WorldPos :type "Vector Structure"))
  (bind _returnvalue (`KismetMathLibrary.FCeil` (/ (`self.BrushRadius`) (`self.CellSize`))))
  (bind _returnvalue_2 (* _returnvalue -1))
  (bind (_gridx _gridy _bvalid) (`self.WorldToGrid` WorldPos))
  (if _bvalid
    (for _index (range _returnvalue_2 (+ _returnvalue 1))
      (for _index_2 (range _returnvalue_2 (+ _returnvalue 1))
        (if (not (> (+ (* _index_2 _index_2) (* _index _index)) (* _returnvalue _returnvalue)))
          (bind _returnvalue_3 (+ _index_2 _gridx))
          (bind _returnvalue_4 (+ _index _gridy))
          (if (and (and (>= _returnvalue_3 0) (< _returnvalue_3 (`self.NumX`))) (and (>= _returnvalue_4 0) (< _returnvalue_4 (`self.NumY`))))
            (bind _returnvalue_5 (+ (* _returnvalue_4 (`self.NumX`)) _returnvalue_3))
            (if (and (`|GetArrayItem` (`self.AllowedMask`) _returnvalue_5) (not (`|GetArrayItem` (`self.VisitedMask`) _returnvalue_5)))
              (`KismetArrayLibrary.Array_Set` (`self.VisitedMask`) _returnvalue_5 true true)
              (set `self.VisitedCount` (+ (`self.VisitedCount`) 1)))))))))

(fn `GetCounts`
  (returns (Allowed :type Integer) (Visited :type Integer))
  (return (`self.AllowedCount`) (`self.VisitedCount`)))

(fn `GridIndexToWorld`
  (params (X :type Integer) (Y :type Integer))
  (returns (WorldLocation :type "Vector Structure"))
  (bind _bounds (`self.Bounds`))
  (bind _cellsize (`self.CellSize`))
  (bind (_returnvalue_x _returnvalue_y) (`KismetMathLibrary.BreakVector` (`BoxComponent.GetScaledBoxExtent` _bounds)))
  (return (`KismetMathLibrary.TransformLocation` (`SceneComponent.K2_GetComponentToWorld` _bounds) (`KismetMathLibrary.MakeVector` (- (* (+ (`KismetMathLibrary.Conv_IntToDouble` X) 0.5) _cellsize) _returnvalue_x) (- (* (+ (`KismetMathLibrary.Conv_IntToDouble` Y) 0.5) _cellsize) _returnvalue_y)))))

(fn `IsHitCleanable`
  (params (Hit :type "HitResult Structure"))
  (returns (ReturnValue :type Boolean))
  (bind _z (.z Hit_ImpactPoint))
  (return (and (and (>= _z (`self.MinZ`)) (<= _z (`self.MaxZ`))) (>= (`KismetMathLibrary.Dot_VectorVector` Hit_ImpactNormal (`KismetMathLibrary.MakeVector` 0.0 0.0 1.0)) (`KismetMathLibrary.DegreesToRadians` (`self.MaxSlopeDeg`))) (or (not (`self.UseTagFilter`)) (`ActorComponent.ComponentHasTag` Hit_HitComponent "Cleanable")))))

(fn `UserConstructionScript`)

(fn `WorldToGrid`
  (params (World :type "Vector Structure"))
  (returns (GridX :type Integer) (GridY :type Integer) (bValid :type Boolean))
  (bind _bounds (`self.Bounds`))
  (bind _cellsize (`self.CellSize`))
  (bind (_returnvalue_x _returnvalue_y) (`KismetMathLibrary.BreakVector` (`BoxComponent.GetScaledBoxExtent` _bounds)))
  (bind (_returnvalue_x_2 _returnvalue_y_2) (`KismetMathLibrary.BreakVector` (`KismetMathLibrary.InverseTransformLocation` (`SceneComponent.K2_GetComponentToWorld` _bounds) World)))
  (bind _returnvalue (`KismetMathLibrary.FFloor` (/ (+ _returnvalue_y_2 _returnvalue_y) _cellsize)))
  (bind _returnvalue_2 (`KismetMathLibrary.FFloor` (/ (+ _returnvalue_x_2 _returnvalue_x) _cellsize)))
  (return _returnvalue_2 _returnvalue (and (and (>= _returnvalue_2 0) (< _returnvalue_2 (`self.NumX`))) (and (>= _returnvalue 0) (< _returnvalue (`self.NumY`))))))