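; BP_EnemyTeleport is an enemy that teleports away when the player touches it, until it runs out of teleports.
; An OverlapDetector overlap with BP_ThirdPersonCharacter moves it to a random reachable navmesh point around the player and increments TeleportCount.
; Once TeleportCount reaches MaxTeleportCount, the next overlap destroys it.
; Tick, throttled by a short Delay, reports its location to BP_ThirdPersonGameMode through HandleEnemyStep.
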(event `self.ReceiveTick`
  (params (DeltaSeconds :type "Float (single-precision)"))
  (`KismetSystemLibrary.Delay` 0.1)
  (bind _asbp_third_person_game_mode (cast `/Game/ThirdPerson/Blueprints/BP_ThirdPersonGameMode` (`GameplayStatics.GetGameMode`)))
  (`/Game/ThirdPerson/Blueprints/BP_ThirdPersonGameMode.HandleEnemyStep` _asbp_third_person_game_mode (`self.K2_GetActorLocation`)))

(event `self.OverlapDetector.OnComponentBeginOverlap`
  (params (OverlappedComponent :type "PrimitiveComponent Object Reference") (OtherActor :type "Actor Object Reference") (OtherComp :type "PrimitiveComponent Object Reference") (OtherBodyIndex :type Integer) (bFromSweep :type Boolean) (SweepResult :type "HitResult Structure (by ref)"))
  ;[1 1 1 0.5] Enemy Teleport Mechanic
  (bind _asbp_third_person_character (cast `/Game/ThirdPerson/Blueprints/BP_ThirdPersonCharacter` OtherActor))
  (if (< (`self.TeleportCount`) (`self.MaxTeleportCount`))
    (`self.K2_SetActorLocation` (`NavigationSystemV1.K2_GetRandomReachablePointInRadius` (`self.K2_GetActorLocation` _asbp_third_person_character) 1000.0 null null) true true)
    (`/Engine/EditorBlueprintResources/StandardMacros.IncrementInt` (`self.TeleportCount`))
    (else
      (`self.K2_DestroyActor`))))

(fn `UserConstructionScript`)