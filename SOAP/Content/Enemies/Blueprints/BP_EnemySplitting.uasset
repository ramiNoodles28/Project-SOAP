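; BP_EnemySplitting is an enemy that splits into two smaller copies when hit.
; Its OverlapDetector reacts to bath bombs, bubble wands, spray bottles and Brush actors, detonating bombs and popping wands.
; A first-generation enemy spawns two second-generation children at offset positions, scaled by ChildScaleMultiplier, then destroys itself.
; Other generations are simply destroyed, so splitting happens only once.
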(event `self.OverlapDetector.OnComponentBeginOverlap`
  (params (OverlappedComponent :type "PrimitiveComponent Object Reference") (OtherActor :type "Actor Object Reference") (OtherComp :type "PrimitiveComponent Object Reference") (OtherBodyIndex :type Integer) (bFromSweep :type Boolean) (SweepResult :type "HitResult Structure (by ref)"))
  (bind _returnvalue (* (`self.EnemyScale`) (`self.ChildScaleMultiplier`)))
  (bind _returnvalue_2 (* (`self.EnemyScale`) (`self.ChildScaleMultiplier`)))
  ;[1 0.9571 0.9671 0.5] Enemy Splitting Mechanic
  (bind _asbp_bath_bomb (cast `/Game/ThirdPerson/Blueprints/Items/BP_BathBomb` OtherActor)
    (:`then`
      (`/Game/ThirdPerson/Blueprints/Items/BP_BathBomb.Detonate` _asbp_bath_bomb))
    (:`CastFailed`
      (bind _asbp_bubble_wand_1 (cast `/Game/ThirdPerson/Blueprints/Items/BP_BubbleWand1` OtherActor)
        (:`then`
          (`/Game/ThirdPerson/Blueprints/Items/BP_BubbleWand1.Pop` _asbp_bubble_wand_1))
        (:`CastFailed`
          (cast `/Game/ThirdPerson/Blueprints/Items/BP_SprayBottles` OtherActor
            (:`then`
              _)
            (:`CastFailed`
              (cast `Brush` OtherActor)))))))
  (if (== (`self.EnemyGeneration`) 1)
    (bind _returnvalue_3 (`|SpawnActorFromClass` "BP_EnemySplitting_C" (`KismetMathLibrary.MakeTransform` (+ (`self.K2_GetActorLocation`) (`KismetMathLibrary.MakeVector` (`self.SpawnOffset`)))) "Undefined" "MultiplyWithRoot" null null))
    (bind _asbp_enemy_splitting (cast `/Game/Enemies/Blueprints/BP_EnemySplitting` _returnvalue_3))
    (set `/Game/Enemies/Blueprints/BP_EnemySplitting.EnemyGeneration` 2 _asbp_enemy_splitting)
    (set `/Game/Enemies/Blueprints/BP_EnemySplitting.EnemyScale` _returnvalue_2 _asbp_enemy_splitting)
    (`self.SetActorScale3D` _asbp_enemy_splitting (`KismetMathLibrary.MakeVector` _returnvalue_2 _returnvalue_2 _returnvalue_2))
    (bind _returnvalue_4 (`|SpawnActorFromClass` "BP_EnemySplitting_C" (`KismetMathLibrary.MakeTransform` (+ (`self.K2_GetActorLocation`) (`KismetMathLibrary.MakeVector` 0.0 -100.0))) "Undefined" "MultiplyWithRoot" null null))
    (bind _asbp_enemy_splitting_2 (cast `/Game/Enemies/Blueprints/BP_EnemySplitting` _returnvalue_4))
    (set `/Game/Enemies/Blueprints/BP_EnemySplitting.EnemyGeneration` 2 _asbp_enemy_splitting_2)
    (set `/Game/Enemies/Blueprints/BP_EnemySplitting.EnemyScale` _returnvalue _asbp_enemy_splitting_2)
    (`self.SetActorScale3D` _asbp_enemy_splitting_2 (`KismetMathLibrary.MakeVector` _returnvalue _returnvalue _returnvalue))
    (`self.K2_DestroyActor`)
    (else
      (`self.K2_DestroyActor`))))

(fn `UserConstructionScript`)