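; Splitter slime enemy that roams to random nearby points and moves toward the player once PawnSensing sees them.
; Overlapping the player while large spawns two copies on opposite sides, with the small-slime flag, mesh and scale changes applied to itself rather than the copies.
; Overlapping while small destroys it.
; HasSplit gates the overlap logic but is never set here, and the SplitterCollision overlap event is empty.
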(event `self.PawnSensing.OnSeePawn`
  (params (Pawn :type "Pawn Object Reference"))
  ; Splitter Enemy Player Tracking
  (set `self.isSeeingPlayer` true)
  (`self.FollowPlayer`))

(event `FollowPlayer`
  ; Splitter Enemy Player Tracking
  (if (`self.isSeeingPlayer`)
    (`|AIMoveTo` self (0.0 0.0 0.0) (`GameplayStatics.GetPlayerCharacter` 0))))

(event `Random Roam`
  ;[0.15 0.1443 0.02335 0.5] Splitter Enemy Movement
  (`|AIMoveTo` self (`NavigationSystemV1.K2_GetRandomReachablePointInRadius` (`self.K2_GetActorLocation`) 1000.0 null null) null
    (:`then`
      (`KismetSystemLibrary.Delay` 5.0)
      (`self.Random Roam`))))

(event `self.ReceiveBeginPlay`
  ;[0.15 0.1443 0.02335 0.5] Splitter Enemy Movement
  (`self.Random Roam`)
  (if (`self.bIsSmallSlime`)
    (`SkeletalMeshComponent.SetSkeletalMeshAsset` (`self.Mesh`) "/Game/Characters/Mannequins/Meshes/SKM_Quinn.SKM_Quinn")
    (`self.SetActorScale3D` (`self.sizeScale`))
    (else
      (`SkeletalMeshComponent.SetSkeletalMeshAsset` (`self.Mesh`) "/Game/Characters/Mannequin_UE4/Meshes/SK_Mannequin.SK_Mannequin"))))

(event `self.ReceiveActorBeginOverlap`
  (params (OtherActor :type "Actor Object Reference"))
  (bind _returnvalue (`self.K2_GetActorLocation`))
  (cast `/Game/ThirdPerson/Blueprints/BP_ThirdPersonCharacter` OtherActor)
  (if (not (`self.bHasSplit`))
    (if (`self.bIsSmallSlime`)
      (`self.K2_DestroyActor`)
      (else
        (bind _returnvalue_2 (`|SpawnActorFromClass` "NewBP_EnemySplitter_C" (`KismetMathLibrary.MakeTransform` (+ _returnvalue (500.0 0.0 0.0)) (`self.K2_GetActorRotation`)) "Undefined" "MultiplyWithRoot" null null))
        (cast `/Game/Enemies/Blueprints/NewBP_EnemySplitter` _returnvalue_2)
        (set `self.bIsSmallSlime` true)
        (`SkeletalMeshComponent.SetSkeletalMeshAsset` (`self.Mesh`) "/Game/Characters/Mannequins/Meshes/SKM_Manny_Simple.SKM_Manny_Simple")
        (`self.SetActorScale3D` (`self.sizeScale`))
        (bind _returnvalue_3 (`|SpawnActorFromClass` "NewBP_EnemySplitter_C" (`KismetMathLibrary.MakeTransform` (+ _returnvalue (-500.0 0.0 0.0)) (`self.K2_GetActorRotation`)) "Undefined" "MultiplyWithRoot" null null))
        (cast `/Game/Enemies/Blueprints/NewBP_EnemySplitter` _returnvalue_3)
        (set `self.bIsSmallSlime` true)
        (`SkeletalMeshComponent.SetSkeletalMeshAsset` (`self.Mesh`) "/Game/Characters/Mannequins/Meshes/SKM_Manny_Simple.SKM_Manny_Simple")
        (`self.SetActorScale3D` (`self.sizeScale`))))))

(event `self.Splitter Collision.OnComponentBeginOverlap`
  (params (OverlappedComponent :type "PrimitiveComponent Object Reference") (OtherActor :type "Actor Object Reference") (OtherComp :type "PrimitiveComponent Object Reference") (OtherBodyIndex :type Integer) (bFromSweep :type Boolean) (SweepResult :type "HitResult Structure (by ref)")))

(fn `UserConstructionScript`)