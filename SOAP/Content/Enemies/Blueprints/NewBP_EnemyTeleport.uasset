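; Enemy that paints a trail as it moves and teleports away when the player character touches it.
; It roams to random reachable points, switching to chasing the player once PawnSensing sees a pawn.
; Each tick, a short downward trace finds the collision UV on BP_Canvas to paint, then reports the hit to the game mode.
; Teleports pick random reachable points under a cooldown, and the enemy destroys itself once its teleport limit is spent.
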(event `Random Roam`
  ;[0.15 0.1443 0.02335 0.5] Teleport Enemy Movement
  (`GameplayStatics.PlaySound2D` "/Game/Audio/Movement/enemy-walkingSound.enemy-walkingSound" 0.3 1.0 0.0 null null)
  (`|AIMoveTo` self (`NavigationSystemV1.K2_GetRandomReachablePointInRadius` (`self.K2_GetActorLocation`) 1000.0 null null) null
    (:`then`
      (`KismetSystemLibrary.Delay` 5.0)
      (`self.Random Roam`))))

(event `self.ReceiveBeginPlay`
  ;[0.15 0.1443 0.02335 0.5] Teleport Enemy Movement
  (`self.Random Roam`))

(event `self.PawnSensing.OnSeePawn`
  (params (Pawn :type "Pawn Object Reference"))
  ; Teleport Enemey Player Tracking
  (set `self.isSeeingPlayer` true)
  (`self.FollowPlayer`))

(event `FollowPlayer`
  ; Teleport Enemey Player Tracking
  (if (`self.isSeeingPlayer`)
    (`GameplayStatics.PlaySound2D` "/Game/Audio/Movement/enemy-walkingSound.enemy-walkingSound" 0.3 1.0 0.0 null null)
    (`|AIMoveTo` self (0.0 0.0 0.0) (`GameplayStatics.GetPlayerCharacter` 0))))

(event `self.ReceiveTick`
  (params (DeltaSeconds :type "Float (single-precision)"))
  (bind _returnvalue (`self.K2_GetActorLocation`))
  ;[0.15 0 0.1023 0.5] Enemy Paint Trail
  (bind _outhit (`KismetSystemLibrary.LineTraceSingle` :`Start` (+ _returnvalue (`KismetMathLibrary.MakeVector` 0.0 0.0 -90.1)) :`End` (+ _returnvalue (`KismetMathLibrary.MakeVector` 0.0 0.0 -93.0)) :`TraceChannel` "TraceTypeQuery1" :`bTraceComplex` true :`bIgnoreSelf` false))
  (bind (_bblockinghit _binitialoverlap _time _distance _location _impactpoint _normal _impactnormal _physmat _hitactor) (`GameplayStatics.BreakHitResult` _outhit))
  (bind _asbp_canvas (cast `/Game/CoverageSys/Blueprints/BP_Canvas` _hitactor))
  (`|ExecutionSequence`
    (:`then_0`
      (`/Game/CoverageSys/Blueprints/BP_Canvas.Paint` _asbp_canvas (`self.T Brush`) (`self.Brush Size`) (`GameplayStatics.FindCollisionUV` _outhit) false))
    (:`then_1`
      (bind _asbp_third_person_game_mode (cast `/Game/ThirdPerson/Blueprints/BP_ThirdPersonGameMode` (`GameplayStatics.GetGameMode`)))
      (`/Game/ThirdPerson/Blueprints/BP_ThirdPersonGameMode.HandlePaintHit` _asbp_third_person_game_mode _impactpoint))))

(event `self.ReceiveActorBeginOverlap`
  (params (OtherActor :type "Actor Object Reference"))
  ;[0 0.0713 0.15 0.5] Enemy Teleporting Mechanic
  (cast `/Game/ThirdPerson/Blueprints/BP_ThirdPersonCharacter` OtherActor)
  (`KismetSystemLibrary.PrintString` "Overlap Successful")
  (`self.TeleportAway`)
  (`GameplayStatics.PlaySound2D` "/Game/Audio/Movement/enemy-teleportSound.enemy-teleportSound" 0.5 1.0 0.0 null null)
  (`KismetSystemLibrary.PrintString` "Bro teleported"))

(event `TeleportAway`
  ;[0 0.0713 0.15 0.5] Enemy Teleporting Mechanic
  (if (`self.CanTeleport`)
    (set `self.CanTeleport` false)
    (if (< (`self.TeleportCount`) (`self.MaxTeleport Count`))
      (bind _returnvalue (`self.K2_GetActorLocation`))
      (bind _randomlocation (`NavigationSystemV1.K2_GetRandomReachablePointInRadius` _returnvalue (`self.TeleportRadius`) null null))
      (`self.K2_SetActorLocation` _randomlocation false true)
      (`/Engine/EditorBlueprintResources/StandardMacros.IncrementInt` (`self.TeleportCount`)
        (:`  `
          (`KismetSystemLibrary.Delay` (`self.TeleportCoolDown`))
          (set `self.CanTeleport` true)))
      (else
        (`self.K2_DestroyActor`)
        (`KismetSystemLibrary.PrintString` "Enemy Destroyed")
        (`GameplayStatics.PlaySound2D` "/Game/Audio/Movement/enemy-teleportSound.enemy-teleportSound" 0.7 1.0 0.0 null null)))))

(fn `UserConstructionScript`)