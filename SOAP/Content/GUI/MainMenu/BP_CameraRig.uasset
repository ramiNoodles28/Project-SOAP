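; BP_CameraRig is a main menu camera rig that offsets and tilts a CineCamera according to the mouse position.
; It normalizes the cursor to a -1 to 1 range across the viewport, then scales it by MaxOffset and MaxRot.
; Interpolation toward these targets runs once on BeginPlay with a fixed delta time, as Tick is empty.
; The location target builds on the stored base location, while the rotation target ignores the stored base rotation.
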(event `self.ReceiveBeginPlay`
  (bind _cinecamera (`self.CineCamera`))
  (bind _cinecamera_2 (`self.CineCamera`))
  (bind (_maxoffset_x _maxoffset_y _maxoffset_z) (`KismetMathLibrary.BreakVector` (`self.MaxOffset`)))
  (bind (_maxrot_roll _maxrot_pitch _maxrot_yaw) (`KismetMathLibrary.BreakRotator` (`self.MaxRot`)))
  (bind _cinecamera_3 (`self.CineCamera`))
  (bind (_sizex _sizey) (`PlayerController.GetViewportSize` (`GameplayStatics.GetPlayerController` 0)))
  (bind _returnvalue (`WidgetLayoutLibrary.GetMousePositionOnViewport`))
  (set `self.BaseLoc` (`SceneComponent.RelativeLocation` _cinecamera))
  (set `self.BaseRot` (`SceneComponent.RelativeRotation` _cinecamera))
  (bind _returnvalue_2 (- (* (/ (`KismetMathLibrary.BreakVector2D` _returnvalue) _sizex) 2.0) 1.0))
  (bind _returnvalue_3 (- (* (/ (`.Y` (`KismetMathLibrary.BreakVector2D` _returnvalue)) _sizey) 2.0) 1.0))
  (set `self.TargetLoc` (+ (`self.BaseLoc`) (`KismetMathLibrary.MakeVector` 0.0 (* _maxoffset_y _returnvalue_2) (* _maxoffset_z _returnvalue_3))))
  (set `self.TargetRot` (`KismetMathLibrary.MakeRotator` (* _returnvalue_2 _maxrot_yaw) (* _returnvalue_3 _maxrot_pitch)))
  (`SceneComponent.K2_SetRelativeLocation` _cinecamera_2 (`KismetMathLibrary.VInterpTo` (`SceneComponent.RelativeLocation` _cinecamera_3) (`self.TargetLoc`) 1.0 (`self.Smooth`)) false false)
  (`SceneComponent.K2_SetRelativeRotation` _cinecamera_2 (`KismetMathLibrary.RInterpTo` (`SceneComponent.RelativeRotation` _cinecamera_3) (`self.TargetRot`) 1.0 (`self.Smooth`)) false false))

(event `self.ReceiveTick`
  (params (DeltaSeconds :type "Float (single-precision)")))

(fn `UserConstructionScript`)