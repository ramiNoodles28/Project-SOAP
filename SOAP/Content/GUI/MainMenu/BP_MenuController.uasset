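; Main menu controller that lets the player click MenuButton actors in the world with the mouse.
; BeginPlay shows the cursor, enables click events and switches input to game and UI.
; Each tick traces under the cursor on the Visibility channel and stores any MenuButton hit as HoveredButton, which is never cleared on a miss.
; Left click checks HoveredButton validity, then calls ExecuteAction on the tick's cast result.
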(event `self.ReceiveBeginPlay`
  (bind _returnvalue (`GameplayStatics.GetPlayerController` 0))
  (set `PlayerController.bShowMouseCursor` true _returnvalue)
  (set `PlayerController.bEnableClickEvents` true _returnvalue)
  (set `PlayerController.bEnableMouseOverEvents` false _returnvalue)
  (`WidgetBlueprintLibrary.SetInputMode_GameAndUIEx` _returnvalue null))

(event `self.ReceiveTick`
  (params (DeltaSeconds :type "Float (single-precision)"))
  (bind _asmenu_button (cast `/Game/GUI/MainMenu/MenuButton` (`.HitActor` (`GameplayStatics.BreakHitResult` (`self.GetHitResultUnderCursorByChannel` (`GameplayStatics.GetPlayerController` 0) "TraceTypeQuery1" true)))))
  (set `self.HoveredButton` _asmenu_button))

(event `Key|LeftMouseButton`
  (params (Key :type "Key Structure"))
  (:`Pressed`
    (if (`KismetSystemLibrary.IsValid` (`self.HoveredButton`))
      (`/Game/GUI/MainMenu/MenuButton.ExecuteAction` (stale `self.ReceiveTick` _asmenu_button)))))

(fn `UserConstructionScript`)