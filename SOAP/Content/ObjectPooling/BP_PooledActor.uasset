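; BP_PooledActor is a pooled actor that tracks whether it is in use.
; BeginPlay and ReturnToPool both call SetInUse with false, and SetInUse only stores the InUse flag.
; Nodes to toggle collision, visibility and tick, and to start a time-to-live timer calling ReturnToPool, exist but are disconnected and never run.
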(event `self.ReceiveBeginPlay`
  (`self.SetInUse` false))

(event `SetInUse`
  (params (InUse :type Boolean))
  ; https://www.youtube.com/watch?v=f797l7YTcgc&t=911s
  (set `self.InUse` InUse))

(event `ReturnToPool`
  ; https://www.youtube.com/watch?v=f797l7YTcgc&t=911s
  (`self.SetInUse` false))

(fn `UserConstructionScript`)